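; BP_Projectile is a projectile actor with a static mesh component that gets propelled forward on launch.
; Launch applies a velocity-change impulse to the mesh along the actor's forward vector, relying on physics rather than a projectile movement component.
; It then calls PrintYourName, which prints the actor's display name to the screen for debugging.
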(fn `Launch`
  (`PrimitiveComponent.AddImpulse` (`self.StaticMeshComponent`) (* (`self.GetActorForwardVector` self) 2500.0) "None" true)
  (`self.Print_Your_Name`))

(fn `Print_Your_Name`
  (`KismetSystemLibrary.PrintString` (`KismetSystemLibrary.GetDisplayName` self)))

(fn `UserConstructionScript`)